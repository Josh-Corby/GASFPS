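; Base gameplay ability for shooting a ranged weapon, handling targeting, fire animation, impact cues and damage.
; The locally controlled client starts weapon targeting, while the ability plays a fire montage on the first-person mesh, falling back to third-person.
; Montage endings end the ability, and a short timer is also set, even without a mesh.
; Returned target data triggers a firing GameplayCue per valid blocking hit, with damage applied only on authority.
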(event `self.K2_ActivateAbility`
  (`|ExecutionSequence`
    (:`then_0`
      (`self.IsLocallyControlled`
        (:`True`
          (`self.StartRangedWeaponTargetting`))))
    (:`then_1`
      (set `self.AvatarActor` (`self.GetAvatarActorFromActorInfo`)))
    (:`then_2`
      (bind _returnvalue (message `GSInventoryInterface.GetFirstPersonMesh` (`self.AvatarActor`)))
      (`/Engine/EditorBlueprintResources/StandardMacros.IsValid` _returnvalue
        (:`Is Valid`
          (`GSAT_PlayMontageForMeshWaitEvent.PlayMontageForMeshAndWaitForEvent` "None" _returnvalue "/Game/ShooterGame/Animations/FPP_Animations/HerroFPP_RifleFire_Montage.HerroFPP_RifleFire_Montage" 1.0 "None" false
            (:`then`
              (`KismetSystemLibrary.K2_SetTimerDelegate` (`|CreateDelegate` :!event `FireComplete`) 0.1))
            (:`OnCompleted`
              (`self.K2_EndAbility` :!label _label))
            (:`OnInterrupted`
              (goto _label))
            (:`OnCancelled`
              (goto _label))))
        (:`Is Not Valid`
          (bind _returnvalue_2 (message `GSInventoryInterface.GetThirdPersonMesh` (`self.AvatarActor`)))
          (`/Engine/EditorBlueprintResources/StandardMacros.IsValid` _returnvalue_2
            (:`Is Valid`
              (`GSAT_PlayMontageForMeshWaitEvent.PlayMontageForMeshAndWaitForEvent` "None" _returnvalue_2 "/Game/ShooterGame/Animations/FPP_Animations/HerroFPP_RifleFire_Montage.HerroFPP_RifleFire_Montage" 1.0 "None" false
                (:`then`
                  (`KismetSystemLibrary.K2_SetTimerDelegate` (`|CreateDelegate` :!event `FireComplete`) 0.1))
                (:`OnCompleted`
                  (`self.K2_EndAbility` :!label _label_2))
                (:`OnInterrupted`
                  (goto _label_2))
                (:`OnCancelled`
                  (goto _label_2))))
            (:`Is Not Valid`
              (`KismetSystemLibrary.K2_SetTimerDelegate` (`|CreateDelegate` :!event `FireComplete`) 0.1))))))))

(event `FireComplete`
  (`self.K2_EndAbility`))

(event `self.OnRangedWeaponTargetDataReady`
  (params (TargetData :type "GameplayAbilityTargetDataHandle Structure (by ref)"))
  (for _index (range (`AbilitySystemBlueprintLibrary.GetDataCountFromTargetData` TargetData))
    (bind _returnvalue (`AbilitySystemBlueprintLibrary.GetHitResultFromTargetData` TargetData _index))
    (bind (_bblockinghit _binitialoverlap _time _distance _location _impactpoint _normal _impactnormal _physmat _hitactor) (`GameplayStatics.BreakHitResult` _returnvalue))
    (if _bblockinghit
      (`/Engine/EditorBlueprintResources/StandardMacros.IsValid` _hitactor
        (:`Is Valid`
          (`self.K2_ExecuteGameplayCueWithParams` (`self.GameplayCueTagFiring`) (`GameplayCueFunctionLibrary.MakeGameplayCueParametersFromHitResult` _returnvalue))
          (`self.K2_HasAuthority`
            (:`True`
              (bind _returnvalue_2 (`AbilitySystemBlueprintLibrary.GetAbilitySystemComponent` _hitactor))
              (`/Engine/EditorBlueprintResources/StandardMacros.IsValid` _returnvalue_2
                (:`Is Valid`
                  (bind _structout (setmembers `DamageEffectParams` :`StructRef` (`self.MakeDamageEffectParamsFromClassDefaults` _hitactor) :`TargetASC` _returnvalue_2))
                  (`GSAbilitySystemLibrary.ApplyDamageEffect` _structout))))))))))