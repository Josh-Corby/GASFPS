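; Gameplay ability that fires a turret shot using ranged weapon targeting.
; On activation, the locally controlled instance starts targeting, the avatar is cached as the owning character, and a short timer ends the ability.
; When target data arrives, each blocking hit prints the actor's name and executes the firing gameplay cue.
; With authority, it applies a damage effect to the first hit actor if that has an Ability System Component.
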(event `self.K2_ActivateAbility`
  (`|ExecutionSequence`
    (:`then_0`
      (`self.IsLocallyControlled`
        (:`True`
          (`self.StartRangedWeaponTargetting`))))
    (:`then_1`
      (bind _asgscharacter_base (cast `GSCharacterBase` (`self.GetAvatarActorFromActorInfo`)))
      (set `self.OwningCharacter` _asgscharacter_base))
    (:`then_2`
      (`KismetSystemLibrary.K2_SetTimerDelegate` (delegate `FireComplete`) 0.1))))

(event `FireComplete`
  (`self.K2_EndAbility`))

(event `self.OnRangedWeaponTargetDataReady`
  (params (TargetData :type "GameplayAbilityTargetDataHandle Structure (by ref)"))
  (bind (_bblockinghit _binitialoverlap _time _distance _location _impactpoint _normal _impactnormal _physmat _hitactor) (`GameplayStatics.BreakHitResult` (`AbilitySystemBlueprintLibrary.GetHitResultFromTargetData` TargetData)))
  (bind _returnvalue (`AbilitySystemBlueprintLibrary.GetAbilitySystemComponent` _hitactor))
  (set `self.GCNParameter` (`GameplayCueFunctionLibrary.MakeGameplayCueParametersFromHitResult` (`AbilitySystemBlueprintLibrary.GetHitResultFromTargetData` TargetData)))
  (for _index (range (`AbilitySystemBlueprintLibrary.GetDataCountFromTargetData` TargetData))
    (bind _returnvalue_2 (`AbilitySystemBlueprintLibrary.GetHitResultFromTargetData` TargetData _index))
    (bind (_bblockinghit_2 _binitialoverlap_2 _time_2 _distance_2 _location_2 _impactpoint_2 _normal_2 _impactnormal_2 _physmat_2 _hitactor_2) (`GameplayStatics.BreakHitResult` _returnvalue_2))
    (if _bblockinghit_2
      (`KismetSystemLibrary.PrintString` (`KismetSystemLibrary.GetDisplayName` _hitactor_2))
      (`self.K2_ExecuteGameplayCueWithParams` (`self.GameplayCueTagFiring`) (`GameplayCueFunctionLibrary.MakeGameplayCueParametersFromHitResult` _returnvalue_2))))
  (`self.K2_HasAuthority`
    (:`True`
      (`/Engine/EditorBlueprintResources/StandardMacros.IsValid` _returnvalue
        (:`Is Valid`
          (bind _structout (setmembers `DamageEffectParams` :`StructRef` (`self.MakeDamageEffectParamsFromClassDefaults` _hitactor) :`TargetASC` _returnvalue))
          (`GSAbilitySystemLibrary.ApplyDamageEffect` _structout))))))