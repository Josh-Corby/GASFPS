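; Interactable sliding door whose open state is driven by the Gameplay Ability System.
; On interaction, the server toggles GE_Door_Open on the door's own ability system component, checking the Object.Door.State.Open tag.
; A listener for that tag's addition and removal triggers OpenDoor and CloseDoor.
; Separate timelines slide the mesh along local Y, each stopping the other and lerping from the current position to handle mid-motion reversals.
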(event `self.ReceiveBeginPlay`
  (bind _tag (`GSAsyncTask_TagAddedRemoved.ListenForGameplayTagAddedOrRemoved` (`AbilitySystemBlueprintLibrary.GetAbilitySystemComponent` self) (`self.In Tags`))
    (:`OnTagAdded`
      (bind _returnvalue (`BlueprintGameplayTagLibrary.MatchesTag` _tag (struct :`TagName` "Object.Door.State.Open") true))
      (if _returnvalue
        (`self.OpenDoor`)))
    (:`OnTagRemoved`
      (if _returnvalue
        (`self.CloseDoor`)))))

(event `GSInteractableInterface.PostInteract`
  (params (InteractingActor :type "Actor Object Reference") (InteractionActor :type "Actor Object Reference"))
  (bind _returnvalue (`AbilitySystemBlueprintLibrary.GetAbilitySystemComponent` self))
  (if (== InteractionActor self)
    (`/Engine/EditorBlueprintResources/ActorMacros.Switch Has Authority`
      (:`Authority`
        (if (`GameplayTagAssetInterface.HasMatchingGameplayTag` (`AbilitySystemBlueprintLibrary.GetAbilitySystemComponent` self) (struct :`TagName` "Object.Door.State.Open"))
          (`AbilitySystemComponent.RemoveActiveGameplayEffect` (`AbilitySystemBlueprintLibrary.GetAbilitySystemComponent` self) (`self.GEDoorOpenHandle`) -1)
          (else
            (bind _returnvalue_2 (`AbilitySystemComponent.BP_ApplyGameplayEffectToSelf` _returnvalue "/Game/Blueprints/AbilitySystem/Effects/GE_Door_Open.GE_Door_Open_C" 0.0 (`AbilitySystemComponent.MakeEffectContext` _returnvalue)))
            (set `self.GEDoorOpenHandle` _returnvalue_2)))))))

(event `OpenDoor`
  (bind _startingtime (`self.StartingTime`))
  (bind (_relativelocation_x _relativelocation_y) (`KismetMathLibrary.BreakVector` (`SceneComponent.RelativeLocation` (`self.DoorMesh`))))
  ;[1 1 1] OpenDoor
  (bind _closedoortimeline (`self.CloseDoorTimeline`)
    (:`then`
      (`TimelineComponent.Stop` _closedoortimeline) ; Stop any current door closing.
    )
    (:`else`
      _))
  (bind _output_get (set `self.DoorStartingRelativeLocationY` _relativelocation_y))
  ;;[0 0 0] Calculate starting time in case door isn't fully closed when trying to open (pressing button again mid-closing).
  (bind _output_get_2 (set `self.StartingTime` (* (`KismetMathLibrary.Abs` (/ _output_get (`self.MaxDoorMovementDistance`))) (`self.TimetoOpenCloseDoor`))))
  (`|ExecutionSequence`
    (:`then_0`
      (bind (_direction _alpha) (`Timeline|OpenDoorTimeline` :`NewTime` _output_get_2 :!via `SetNewTime` :!label _label)
        (:`Update`
          (`SceneComponent.K2_SetRelativeLocation` (`self.DoorMesh`) (`KismetMathLibrary.MakeVector` 0.0 (`KismetMathLibrary.Lerp` (`self.DoorStartingRelativeLocationY`) -140.0 (/ (- _alpha _startingtime) (- (`self.TimetoOpenCloseDoor`) _startingtime)))) false false))))
    (:`then_1`
      (goto _label))))

(event `CloseDoor`
  (bind _startingtime (`self.StartingTime`))
  (bind (_relativelocation_x _relativelocation_y) (`KismetMathLibrary.BreakVector` (`SceneComponent.RelativeLocation` (`self.DoorMesh`))))
  ;[1 1 1] CloseDoor
  (bind _opendoortimeline (`self.OpenDoorTimeline`)
    (:`then`
      (`TimelineComponent.Stop` _opendoortimeline) ; Stop any current door opening.
    )
    (:`else`
      _))
  (bind _output_get (set `self.DoorStartingRelativeLocationY` _relativelocation_y))
  ;;[0 0 0] Calculate starting time in case door isn't fully opened when trying to close (pressing button again mid-opening).
  (set `self.StartingTime` (* (- (`KismetMathLibrary.Abs` (/ _output_get (`self.MaxDoorMovementDistance`))) 1.0) (`self.TimeToOpenCloseDoor`)))
  (`|ExecutionSequence`
    (:`then_0`
      (bind (_direction _alpha) (`Timeline|CloseDoorTimeline` :!via `SetNewTime` :!label _label_2)
        (:`Update`
          (`SceneComponent.K2_SetRelativeLocation` (`self.DoorMesh`) (`KismetMathLibrary.MakeVector` 0.0 (`KismetMathLibrary.Lerp` (`self.DoorStartingRelativeLocationY`) 0.0 (/ (- _alpha _startingtime) (- (`self.TimetoOpenCloseDoor`) _startingtime)))) false false))))
    (:`then_1`
      (goto _label_2))))

(fn `GetInteractionDuration`
  (params (InteractionActor :type "Actor Object Reference"))
  (returns (ReturnValue :type "Float (single-precision)"))
  (return 0.0))

(fn `GetPostInteractSyncType`
  (params (InteractionActor :type "Actor Object Reference"))
  (returns (bShouldSync :type Boolean) (Type :type "EAbilityTaskNetSyncType Enum"))
  (return false "BothWait"))

(fn `GetPreInteractSyncType`
  (params (InteractionActor :type "Actor Object Reference"))
  (returns (bShouldSync :type Boolean) (Type :type "EAbilityTaskNetSyncType Enum"))
  (return false "BothWait"))

(fn `IsAvailableForInteraction`
  (params (InteractionActor :type "Actor Object Reference"))
  (returns (ReturnValue :type Boolean))
  (return true))

(fn `UserConstructionScript`)