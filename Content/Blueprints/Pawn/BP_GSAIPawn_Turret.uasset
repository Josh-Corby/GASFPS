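; Turret AI pawn that uses the Gameplay Ability System to fire at detected targets.
; It grants itself GA_Shoot_Turret on BeginPlay.
; Target detection starts a short wind-up timer, unless one is already preparing or firing, which then hands off to a rapid looping timer that tries to activate the shoot ability.
; Losing the target clears both timers.
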(event `self.ReceiveBeginPlay`
  (`AbilitySystemComponent.K2_GiveAbility` (`self.AbilitySystemComponent`) "/Game/Blueprints/AbilitySystem/Abilities/GA_Shoot_Turret.GA_Shoot_Turret_C" 1 -1))

(event `self.TargetDetected`
  (params (TargetActor :type "Actor Object Reference"))
  (`parent.TargetDetected` TargetActor)
  (if (not (or (`KismetSystemLibrary.K2_IsValidTimerHandle` (`self.FiringHandle`)) (`KismetSystemLibrary.K2_IsValidTimerHandle` (`self.PrepareToFireHandle`))))
    (bind _returnvalue (`KismetSystemLibrary.K2_SetTimerDelegate` (delegate `PrepareToFire`) 1.0))
    (set `self.PrepareToFireHandle` _returnvalue)))

(event `PrepareToFire`
  (bind _returnvalue (`KismetSystemLibrary.K2_SetTimerDelegate` (delegate `Shoot`) 0.1 true))
  (set `self.FiringHandle` _returnvalue)
  (`KismetSystemLibrary.K2_ClearAndInvalidateTimerHandle` (`self.PrepareToFireHandle`)))

(event `Shoot`
  (`AbilitySystemComponent.TryActivateAbilityByClass` (`self.AbilitySystemComponent`) "/Game/Blueprints/AbilitySystem/Abilities/GA_Shoot_Turret.GA_Shoot_Turret_C" false))

(event `self.TargetLost`
  (`KismetSystemLibrary.K2_ClearAndInvalidateTimerHandle` (`self.FiringHandle`))
  (`KismetSystemLibrary.K2_ClearAndInvalidateTimerHandle` (`self.PrepareToFireHandle`)))

(fn `UserConstructionScript`
  (`parent.UserConstructionScript`))